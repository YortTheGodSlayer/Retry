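; Enemy AI Blueprint that chases the player, deals damage on reaching them and destroys itself when Health drops below one.
; PawnSensing sight or hearing sets IsSeeingPlayer, never cleared here, and calls FollowPlayer to run AIMoveTo toward player zero.
; Successful moves apply Damage.
; The attack montage is gated by CanAttack, which FollowPlayer clears before moving; death sets IsDead to false before destroying the actor.
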(event OnSeePawn(PawnSensing)
  (params (Pawn :type Pawn%20Object%20Reference))
  ;[1 1 1] Comment
  (Variables|Default|SetisSeeingPlayer? true)
  (CallFunction|FollowPlayer))

(event OnHearNoise(PawnSensing)
  (params (Instigator :type Pawn%20Object%20Reference) (Location :type Vector%20%28by%20ref%29 :default "0, 0, 0") (Volume :type Float%20%28single-precision%29))
  ;[1 1 1] Comment
  (Variables|Default|SetisSeeingPlayer? true)
  (CallFunction|FollowPlayer))

(event Custom|FollowPlayer
  (bind _returnvalue (Game|GetPlayerCharacter 0))
  ;[1 1 1] Comment
  (Variables|Default|SetcanAttack? false)
  (if (Variables|Default|GetisSeeingPlayer?)
    (AI|AIMoveTo self "0, 0, 0" _returnvalue 7e+01 false
      (:then
        (if (Variables|Default|GetcanAttack?)
          (Variables|Default|SetcanAttack? false)
          (bind _returnvalue_2 (Animation|PlayAnimMontage "/Game/FirstPerson/Animations/FirstPersonFire_Montage.FirstPersonFire_Montage" 1.0 "None"))
          (Utilities|FlowControl|Delay _returnvalue_2)
          (Variables|Default|SetcanAttack? true)))
      (:OnSuccess
        (Game|Damage|ApplyDamage _returnvalue (Variables|Default|GetDamage) 0 0)))))

(event EventBeginPlay)

(event Collision|EventActorBeginOverlap
  (params (OtherActor :type Actor%20Object%20Reference)))

(event EventTick
  (params (DeltaSeconds :type Float%20%28single-precision%29)))

(event Game|Damage|EventAnyDamage
  (params (Damage :type Float%20%28single-precision%29) (DamageType :type Damage%20Type%20Object%20Reference) (InstigatedBy :type Controller%20Object%20Reference) (DamageCauser :type Actor%20Object%20Reference))
  ;[1 1 1] Take Damage
  (Variables|Default|SetHealth (- (Variables|Default|GetHealth) Damage))
  (if (< (Variables|Default|GetHealth) 1.0)
    (Variables|Default|SetisDead? false)
    (Actor|DestroyActor)))

(fn ConstructionScript)